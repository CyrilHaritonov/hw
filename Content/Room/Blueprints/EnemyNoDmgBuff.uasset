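; EnemyNoDmgBuff is a potion pickup that grants temporary invincibility to damage from static enemies.
; On BeginPlay it caches the GlobalState actor found in the level.
; The first character overlap with its Box sets IsInvinsible on GlobalState, hides the pickup and starts a timer of LengthOfNoDmgEffect.
; The hidden actor stays alive so the timer can clear the flag and print a debug message.
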(event OnComponentBeginOverlap(Box)
  (params (OverlappedComponent :type Primitive%20Component%20Object%20Reference) (OtherActor :type Actor%20Object%20Reference) (OtherComp :type Primitive%20Component%20Object%20Reference) (OtherBodyIndex :type Integer) (bFromSweep :type Boolean) (SweepResult :type Hit%20Result%20Structure%20%28by%20ref%29))
  ;[1 1 1] При поднятии зелья включаем переменную неуязвимости к урону от статических врагов
  (Utilities|Casting|CastToBP_ThirdPersonCharacter OtherActor)
  (Utilities|FlowControl|DoOnce false
    (:Completed
      (Variables|/Game/Room/Blueprints/GlobalState.GlobalState_C|SetIsInvinsible (Variables|Default|GetGlobalState) true)
      (Utilities|Time|SetTimerbyEvent (delegate Custom|Set%20timeout) (Variables|/Game/Room/Blueprints/PDA_Data.PDA_Data_C|GetLengthOfNoDmgEffect (Variables|Default|GetVariables)))
      (Rendering|SetActorHiddenInGame true))))

(event Custom|Set%20timeout
  ;[1 1 1] При поднятии зелья включаем переменную неуязвимости к урону от статических врагов
  (Variables|/Game/Room/Blueprints/GlobalState.GlobalState_C|SetIsInvinsible (Variables|Default|GetGlobalState) false)
  (Development|PrintString "Set invincibility back"))

(event Custom|GetGlobalState
  ;[1 1 1] Получаем доступ к глобальным переменным
  (bind _outactors (Actor|GetAllActorsOfClass "/Game/Room/Blueprints/GlobalState.GlobalState_C"))
  (Variables|Default|SetGlobalState (Utilities|Array|Get(acopy) _outactors)))

(event EventBeginPlay
  (CallFunction|GetGlobalState))

(fn ConstructionScript)