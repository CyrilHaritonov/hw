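; Enemy damage zone that periodically hurts player characters standing inside its Box trigger.
; Box overlap events add BP_ThirdPersonCharacter actors to an ActorsToDamage array and remove them when they leave.
; A looping timer started on BeginPlay applies damage to every tracked actor, unless the GlobalState actor, fetched via GetAllActorsOfClass, flags invincibility.
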(event OnComponentBeginOverlap(Box)
  (params (OverlappedComponent :type Primitive%20Component%20Object%20Reference) (OtherActor :type Actor%20Object%20Reference) (OtherComp :type Primitive%20Component%20Object%20Reference) (OtherBodyIndex :type Integer) (bFromSweep :type Boolean) (SweepResult :type Hit%20Result%20Structure%20%28by%20ref%29))
  ;[1 1 1] Добавляем актора в массив акторов которые находятся в тригере
  (bind _asbp_third_person_character (Utilities|Casting|CastToBP_ThirdPersonCharacter OtherActor))
  (Utilities|IsValid _asbp_third_person_character
    (:Is%20Valid
      (Utilities|Array|Add (Variables|Default|GetActorsToDamage) _asbp_third_person_character))))

(event OnComponentEndOverlap(Box)
  (params (OverlappedComponent :type Primitive%20Component%20Object%20Reference) (OtherActor :type Actor%20Object%20Reference) (OtherComp :type Primitive%20Component%20Object%20Reference) (OtherBodyIndex :type Integer))
  (bind _actorstodamage (Variables|Default|GetActorsToDamage))
  (bind _returnvalue (Utilities|Array|FindItem _actorstodamage OtherActor))
  ;[1 1 1] Удаляем актора из массива акторов, которым должен наносится урон, когда актор покидает триггер
  (if (>= _returnvalue 0)
    (Utilities|Array|RemoveIndex (Variables|Default|GetActorsToDamage) _returnvalue)))

(event Custom|ApplyDamage
  ;[1 1 1] Наносим урон, кажому актору, который находится в данный момент в тригере
  (for _array_element (Variables|Default|GetActorsToDamage)
    (if (not (Variables|/Game/Room/Blueprints/GlobalState.GlobalState_C|GetIsInvinsible (Variables|Default|GetGlobalState)))
      (Game|Damage|ApplyDamage _array_element (Variables|/Game/Room/Blueprints/PDA_Data.PDA_Data_C|GetEnemyDamage (Variables|Default|GetVariables)) 0 0 "/Script/Engine.DamageType"))))

(event Custom|GetGlobalState
  ;[1 1 1] Получаем доступ к глобальным переменным
  (bind _outactors (Actor|GetAllActorsOfClass "/Game/Room/Blueprints/GlobalState.GlobalState_C"))
  (Variables|Default|SetGlobalState (Utilities|Array|Get(acopy) _outactors)))

(event EventBeginPlay
  ;[1 1 1] Наносим урон, кажому актору, который находится в данный момент в тригере
  (CallFunction|GetGlobalState)
  (Utilities|Time|SetTimerbyEvent (delegate Custom|ApplyDamage) (Variables|/Game/Room/Blueprints/PDA_Data.PDA_Data_C|GetDamageDelta (Variables|Default|GetVariables)) true))

(fn ConstructionScript)