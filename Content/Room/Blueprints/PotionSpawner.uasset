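; Room spawner actor that may place one buff, debuff or random potion at its own location on BeginPlay.
; It fetches the GlobalState actor and proceeds only while the current room number does not exceed the maximum.
; Chained random rolls, scaled by difficulty, must beat per-type thresholds, tried in order: enemy slow, enemy no-damage, self-slow, random potion.
; The first success spawns that class; if all fail, nothing spawns.
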(event Custom|GetGlobalState
  ;[1 1 1] Получаем доступ к глобальным переменным
  (bind _outactors (Actor|GetAllActorsOfClass "/Game/Room/Blueprints/GlobalState.GlobalState_C"))
  (Variables|Default|SetGlobalState (Utilities|Array|Get(acopy) _outactors)))

(event EventBeginPlay
  (bind _returnvalue (Math|Random|RandomFloatinRange 0.0 1.0))
  (bind _returnvalue_2 (Transformation|GetActorLocation))
  (bind _globalstate (Variables|Default|GetGlobalState))
  (bind _globalstate_2 (Variables|Default|GetGlobalState))
  (bind _returnvalue_3 (Math|Conversions|ToTransform(Vector) _returnvalue_2))
  (bind _currentdifficulty (Variables|/Game/Room/Blueprints/GlobalState.GlobalState_C|GetCurrentDifficulty _globalstate))
  (bind _returnvalue_4 (* _returnvalue _currentdifficulty))
  ;[1 1 1] Роллим шанс спавна, если прокнуло, то спавним нужный бафф/дебафф, в зависимости от выпавшего числа, на месте спавнера
  (CallFunction|GetGlobalState)
  (Math|Integer|CompareInt (Variables|/Game/Room/Blueprints/GlobalState.GlobalState_C|GetCurrentRoomNumber _globalstate_2) (Variables|/Game/Room/Blueprints/GlobalState.GlobalState_C|GetMaxRoomNumber _globalstate_2)
    (:==
      _)
    (:<
      _))
  (if true
    (if (> _returnvalue_4 (Variables|/Game/Room/Blueprints/PDA_Data.PDA_Data_C|GetSpawnChanceOfSlowInSpawner (Variables|Default|GetVariables)))
      (Game|SpawnActorfromClass "/Game/Room/Blueprints/EnemySlowBuff.EnemySlowBuff_C" _returnvalue_3 "Undefined" "MultiplyWithRoot" 0 0)
      (elif (> _returnvalue_4 (Variables|/Game/Room/Blueprints/PDA_Data.PDA_Data_C|GetSpawnChanceOfFazeInSpawner (Variables|Default|GetVariables)))
        (Game|SpawnActorfromClass "/Game/Room/Blueprints/EnemyNoDmgBuff.EnemyNoDmgBuff_C" _returnvalue_3 "Undefined" "MultiplyWithRoot" 0 0)
        (elif (> _returnvalue_4 (Variables|/Game/Room/Blueprints/PDA_Data.PDA_Data_C|GetSpawnChanceOfDebuffInSpawner (Variables|Default|GetVariables)))
          (Game|SpawnActorfromClass "/Game/Room/Blueprints/SlowYourselfDebuff.SlowYourselfDebuff_C" _returnvalue_3 "Undefined" "MultiplyWithRoot" 0 0)
          (elif (> _returnvalue_4 (Variables|/Game/Room/Blueprints/PDA_Data.PDA_Data_C|GetSpawnChanceOfRandomInSpawner (Variables|Default|GetVariables)))
            (Game|SpawnActorfromClass "/Game/Room/Blueprints/RandomPotion.RandomPotion_C" _returnvalue_3 "Undefined" "MultiplyWithRoot" 0 0)))))))

(fn ConstructionScript)