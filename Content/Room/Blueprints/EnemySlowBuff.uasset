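; EnemySlowBuff is a one-time pickup potion that temporarily slows enemies when the third-person character overlaps its box.
; On BeginPlay it caches the GlobalState actor, whose shared MovingEnemySpeed variable it overwrites with the slowed value on pickup; a comment describes that variable as a timeline length.
; The actor then hides itself rather than being destroyed, and a timer event later restores the default speed.
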(event OnComponentBeginOverlap(Box)
  (params (OverlappedComponent :type Primitive%20Component%20Object%20Reference) (OtherActor :type Actor%20Object%20Reference) (OtherComp :type Primitive%20Component%20Object%20Reference) (OtherBodyIndex :type Integer) (bFromSweep :type Boolean) (SweepResult :type Hit%20Result%20Structure%20%28by%20ref%29))
  (bind _variables (Variables|Default|GetVariables))
  ;[1 1 1] При подбирании зелья замедления врагов, меняем глобальную переменную длинны таймлайна, после чего ставим таймер чтобы поменять ее обратно
  (Utilities|Casting|CastToBP_ThirdPersonCharacter OtherActor)
  (Utilities|FlowControl|DoOnce false
    (:Completed
      (Variables|/Game/Room/Blueprints/GlobalState.GlobalState_C|SetMovingEnemySpeed (Variables|Default|GetGlobalState) (Variables|/Game/Room/Blueprints/PDA_Data.PDA_Data_C|GetSlowedEnemySpeed _variables))
      (Utilities|Time|SetTimerbyEvent (delegate Custom|Set%20timeout) (Variables|/Game/Room/Blueprints/PDA_Data.PDA_Data_C|GetLengthOfEnemySlowEffect _variables))
      (Rendering|SetActorHiddenInGame true))))

(event Custom|Set%20timeout
  (bind _globalstate (Variables|Default|GetGlobalState))
  ;[1 1 1] При подбирании зелья замедления врагов, меняем глобальную переменную длинны таймлайна, после чего ставим таймер чтобы поменять ее обратно
  (Variables|/Game/Room/Blueprints/GlobalState.GlobalState_C|SetMovingEnemySpeed _globalstate (Variables|/Game/Room/Blueprints/GlobalState.GlobalState_C|GetMovingEnemySpeedDefault _globalstate))
  (Development|PrintString "Set speed of enemies back"))

(event Custom|GetGlobalState
  ;[1 1 1] Получаем доступ к глобальным переменным
  (bind _outactors (Actor|GetAllActorsOfClass "/Game/Room/Blueprints/GlobalState.GlobalState_C"))
  (Variables|Default|SetGlobalState (Utilities|Array|Get(acopy) _outactors)))

(event EventBeginPlay
  (CallFunction|GetGlobalState))

(fn ConstructionScript)