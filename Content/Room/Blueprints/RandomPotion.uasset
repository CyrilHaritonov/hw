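; Random potion spawner that turns into a hidden buff or debuff pickup when the player character enters its trigger box.
; A one-time overlap runs cascading random rolls for enemy slow, enemy no-damage, then self-slow, each succeeding when the roll exceeds its chance variable, so higher values make it rarer.
; A success spawns that actor invisible in place and hides the spawner; if all fail, nothing spawns.
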(event OnComponentBeginOverlap(Box)
  (params (OverlappedComponent :type Primitive%20Component%20Object%20Reference) (OtherActor :type Actor%20Object%20Reference) (OtherComp :type Primitive%20Component%20Object%20Reference) (OtherBodyIndex :type Integer) (bFromSweep :type Boolean) (SweepResult :type Hit%20Result%20Structure%20%28by%20ref%29))
  (bind _returnvalue (Math|Random|RandomFloatinRange 0.0 1.0))
  (bind _returnvalue_2 (Transformation|GetActorLocation))
  (bind _returnvalue_3 (Math|Conversions|ToTransform(Vector) _returnvalue_2))
  ;[1 1 1] Спавним рандомное зелье в невидимом состоянии при срабатывании тригера, а сам спавнер делаем невидимым
  (Utilities|Casting|CastToBP_ThirdPersonCharacter OtherActor)
  (Utilities|FlowControl|DoOnce false
    (:Completed
      (if (> _returnvalue (Variables|/Game/Room/Blueprints/PDA_Data.PDA_Data_C|GetSpawnChanceOfSlowInRandom (Variables|Default|GetVariables)))
        (bind _returnvalue_4 (Game|SpawnActorfromClass "/Game/Room/Blueprints/EnemySlowBuff.EnemySlowBuff_C" _returnvalue_3 "Undefined" "MultiplyWithRoot" 0 0))
        (Rendering|SetVisibility (Variables|/Game/Room/Blueprints/EnemySlowBuff.EnemySlowBuff_C|GetDefaultSceneRoot _returnvalue_4) false true)
        (Development|SetHiddeninGame (Variables|Default|GetDefaultSceneRoot) true true :!label _label)
        (elif (> _returnvalue (Variables|/Game/Room/Blueprints/PDA_Data.PDA_Data_C|GetSpawnChanceOfFazeInRandom (Variables|Default|GetVariables)))
          (bind _returnvalue_5 (Game|SpawnActorfromClass "/Game/Room/Blueprints/EnemyNoDmgBuff.EnemyNoDmgBuff_C" _returnvalue_3 "Undefined" "MultiplyWithRoot" 0 0))
          (Rendering|SetVisibility (Variables|/Game/Room/Blueprints/EnemyNoDmgBuff.EnemyNoDmgBuff_C|GetDefaultSceneRoot _returnvalue_5) false true)
          (goto _label)
          (elif (> _returnvalue (Variables|/Game/Room/Blueprints/PDA_Data.PDA_Data_C|GetSpawnChanceOfDebuffInRandom (Variables|Default|GetVariables)))
            (bind _returnvalue_6 (Game|SpawnActorfromClass "/Game/Room/Blueprints/SlowYourselfDebuff.SlowYourselfDebuff_C" _returnvalue_3 "Undefined" "MultiplyWithRoot" 0 0))
            (Rendering|SetVisibility (Variables|/Game/Room/Blueprints/SlowYourselfDebuff.SlowYourselfDebuff_C|GetDefaultSceneRoot _returnvalue_6) false true)
            (goto _label)))))))

(fn ConstructionScript)