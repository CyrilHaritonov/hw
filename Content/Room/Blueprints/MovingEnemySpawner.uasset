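; Room spawner Blueprint that may spawn an Enemy on BeginPlay and send it moving along its spline, skipping the final room.
; Spawn chance is a coefficient times the current difficulty read from the GlobalState actor.
; A self-restarting Timeline sets the enemy's location by spline distance and its rotation from the tangent, looping from the start.
; Tick continually sets the Timeline play rate to the global moving-enemy speed.
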(event Custom|PlayTimeline
  (bind _spline (Variables|Default|GetSpline))
  (bind _actor (Variables|Default|GetActor))
  ;[1 1 1] Двигаем противника по заданному сплайну
  (bind _newtrack_0 (Timeline|Timeline PlayFromStart)
    (:Update
      (Transformation|SetActorLocation _actor (Spline|GetLocationatDistanceAlongSpline (Variables|Default|GetSpline) (Math|Float|Lerp 0.0 (Spline|GetDistanceAlongSplineatSplinePoint _spline (- (Spline|GetNumberOfSplinePoints _spline) 1)) _newtrack_0) "World") false false)
      (Transformation|SetActorRotation _actor (Math|Conversions|RotationFromXVector (Spline|GetTangentatDistanceAlongSpline (Variables|Default|GetSpline) (Math|Float|Lerp 0.0 (Spline|GetDistanceAlongSplineatSplinePoint _spline (- (Spline|GetNumberOfSplinePoints _spline) 1)) _newtrack_0) "World"))))
    (:Finished
      (CallFunction|PlayTimeline))))

(event Custom|GetGlobalState
  ;[1 1 1] Доступ к глобальным переменным
  (bind _outactors (Actor|GetAllActorsOfClass "/Game/Room/Blueprints/GlobalState.GlobalState_C"))
  (Variables|Default|SetGlobalState (Utilities|Array|Get(acopy) _outactors)))

(event EventBeginPlay
  (bind _globalstate (Variables|Default|GetGlobalState))
  ;[1 1 1] Берем сложность из глобальной переменной и на ее основе считаем шанс спавна, если прокнул шанс, то спавним и начинаем движение по таймлайну, если комната конечная то не спавним
  (CallFunction|GetGlobalState)
  (if (not (== (- (Variables|/Game/Room/Blueprints/GlobalState.GlobalState_C|GetCurrentRoomNumber _globalstate) 1) (Variables|/Game/Room/Blueprints/GlobalState.GlobalState_C|GetMaxRoomNumber _globalstate)))
    (if (< (Math|Random|RandomFloatinRange 0.0 1.0) (* (Variables|/Game/Room/Blueprints/PDA_Data.PDA_Data_C|GetMovingEnemySpawnCoefficient (Variables|Default|GetVariables)) (Variables|/Game/Room/Blueprints/GlobalState.GlobalState_C|GetCurrentDifficulty (Variables|Default|GetGlobalState))))
      (bind _returnvalue (Game|SpawnActorfromClass (Variables|Default|GetEnemy) (Transformation|GetWorldTransform (Variables|Default|GetSpline)) "Undefined" "MultiplyWithRoot" 0 0))
      (Variables|Default|SetActor _returnvalue)
      (CallFunction|PlayTimeline))))

(event EventTick
  (params (DeltaSeconds :type Float%20%28single-precision%29))
  ;[1 1 1] Выставялем нужную скорость врагов, каждый кадр
  (Components|Timeline|SetPlayRate (Variables|Default|GetTimeline) (Variables|/Game/Room/Blueprints/GlobalState.GlobalState_C|GetMovingEnemySpeed (Variables|Default|GetGlobalState))))

(fn ConstructionScript)